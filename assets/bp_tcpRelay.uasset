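; TCP relay Blueprint that bridges a local Python process and a pawn in the level, exchanging float arrays as string messages.
; On BeginPlay it sizes both arrays, targets the first Bp_pythonPawn instance and connects to a localhost socket.
; Each Tick parses the latest message into floats for the pawn via a Blueprint interface, then serializes the pawn's returned floats back over TCP, printing both messages for debugging.
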(event `self.ReceiveBeginPlay`
  (`|ExecutionSequence`
    (:`then_0`
      ; Make msg_in array (from Python)
      (`KismetArrayLibrary.Array_Resize` (`self.floats_in`) (`self.num_fields_in`))
      ; Make msg_out array (to Python)
      (`KismetArrayLibrary.Array_Resize` (`self.floats_out`) (`self.num_fields_out`))
      ; Identify pythonPawn or custom actor class (selects first instance) as relay target
      (bind _returnvalue (`GameplayStatics.GetActorOfClass` "/Game/custom/bp_pythonPawn.bp_pythonPawn_C"))
      (set `self.send_to` _returnvalue))
    (:`then_1`
      (`self.Connect` "127.0.0.1" 1234 (delegate `Disconnected`) (delegate `Connected`) (delegate `ReceivedMessage`)))))

(event `Disconnected`
  (params (ConnectionId :type Integer))
  (`self.Print Disconnected`))

(event `/Game/custom/bpi_relay.Relay TCP Data`
  (params (floats :type "Array of Float (double-precision) (by ref)"))
  ; Update 'floats_out' when "Send To" actor rreturns data through the blueprint interface
  (set `self.floats_out` floats))

(event `Connected`
  (params (ConnectionId :type Integer))
  (`self.Print Connected`))

(event `ReceivedMessage`
  (params (ConnectionId :type Integer) (Message :type "Array of Byte (by ref)"))
  (bind _returnvalue (`self.Message_ReadString` Message (`KismetArrayLibrary.Array_Length` Message)))
  (set `self.msg_in` _returnvalue))

(event `Send Data to Actor`
  ; Send parsed 'floats_in' to 'Send To' actor through the blueprint inteface
  (message `/Game/custom/bpi_relay.Relay TCP Data` (`self.send_to`) (`self.floats_in`)))

(event `self.ReceiveTick`
  (params (DeltaSeconds :type "Float (single-precision)"))
  ; Convert Message In string to Floats In array and send to target Actor
  (bind _updated_floats_in (`self.Parse Message to Floats` (`self.msg_in`) (`self.floats_in`)))
  (set `self.floats_in` _updated_floats_in)
  (`self.Send Data to Actor`)
  ; Convert Message Out string to Floats In array and send to Actor
  (bind _as_string (`self.Parse Floats to Message` (`self.floats_out`)))
  (bind _output_get (set `self.msg_out` _as_string))
  (`self.SendData` 0 (`self.Conv_StringToBytes` _output_get))
  (`self.Print Message IO` true true) ; Toggle messages IO display
)

(fn `Parse Floats to Message`
  (params (`Floats to Send` :type "Array of Float (double-precision)"))
  (returns (`As String` :type String))
  (locals (String_Array :type "Array of String"))
  (for _array_element `Floats to Send`
    (`KismetArrayLibrary.Array_Add` (`local.String_Array`) (`KismetStringLibrary.Conv_DoubleToString` _array_element)))
  (return (`KismetStringLibrary.JoinStringArray` (`local.String_Array`))))

(fn `Parse Message to Floats`
  (params (`Message In String` :type String) (`Floats In Array` :type "Array of Float (double-precision)"))
  (returns (`Updated Floats_In` :type "Array of Float (double-precision)"))
  (locals (`New Floats In` :type "Array of Float (double-precision)"))
  ; On event tick, read latest 'msg_in', split by space, update 'floats in'
  (for (_array_element _array_index) (`KismetStringLibrary.ParseIntoArray` `Message In String`)
    (`KismetArrayLibrary.Array_Set` `Floats In Array` _array_index (`KismetStringLibrary.Conv_StringToDouble` _array_element)))
  (return (`local.Floats In Array`)))

(fn `Print Array Info`
  (`KismetSystemLibrary.PrintString` (`KismetStringLibrary.Concat_StrStr` "TCP Message In Length:  " (`KismetStringLibrary.Conv_IntToString` (`KismetArrayLibrary.Array_Length` (`self.floats_in`)))) true true (struct :`R` 1.0 :`G` 0.35484 :`A` 1.0))
  (`KismetSystemLibrary.PrintString` (`KismetStringLibrary.Concat_StrStr` "Msg Out LeTCP Message In Length: " (`KismetStringLibrary.Conv_IntToString` (`KismetArrayLibrary.Array_Length` (`self.floats_out`)))) true true (struct :`R` 1.0 :`B` 0.045854 :`A` 1.0)))

(fn `Print Message IO`
  (params (`Show Message In` :type Boolean) (`Show Message Out` :type Boolean))
  (`|ExecutionSequence`
    (:`then_0`
      (if `Show Message In`
        ; Print Message In
        (`KismetSystemLibrary.PrintString` (`KismetStringLibrary.Concat_StrStr` "Msg In:" " " (`self.msg_in`)) true true (struct :`R` 0.204916 :`G` 0.63125 :`A` 1.0) 0.016667)))
    (:`then_1`
      (if `Show Message Out`
        ; Print Message Out
        (`KismetSystemLibrary.PrintString` (`KismetStringLibrary.Concat_StrStr` "Msg Out:" " " (`self.msg_out`)) true true (struct :`G` 1.0 :`B` 0.192037 :`A` 1.0) 0.016667)))))

(fn `UserConstructionScript`)